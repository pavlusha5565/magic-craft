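; BP_MCPlayerHUD is a player HUD Blueprint that owns the inventory widget.
; It creates WB_Inventory on BeginPlay and keeps a reference to it.
; SetVisibilityInventory toggles the widget on and off the viewport, syncs the mouse cursor and move-input blocking to the open state, and calls SetFocus on the widget.
; A SetVisibilityInventory call in the event graph is unconnected, so this Blueprint never triggers the toggle itself.
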(event `self.ReceiveBeginPlay`
  (bind _returnvalue (`|CreateWidget` "/Game/UI/Inventory/WB_Inventory.WB_Inventory_C"))
  (set `self.WB_Inventory` _returnvalue))

(fn `SetVisibilityInventory`
  (bind _returnvalue (`GameplayStatics.GetPlayerController` 0))
  (bind _wb_inventory (`self.WB_Inventory`))
  (if (not (`self.IsInventoryOpen`))
    (`UserWidget.AddToViewport` _wb_inventory 0)
    (set `self.IsInventoryOpen` true)
    (else
      (`Widget.RemoveFromParent` _wb_inventory)
      (set `self.IsInventoryOpen` false)))
  (bind _output_get (set `PlayerController.bShowMouseCursor` (`self.IsInventoryOpen`) _returnvalue))
  (`Controller.SetIgnoreMoveInput` _returnvalue _output_get)
  (`Widget.SetFocus` (`self.WB_Inventory`)))

(fn `UserConstructionScript`)